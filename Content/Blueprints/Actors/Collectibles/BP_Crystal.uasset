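; Collectible crystal actor that flies to the player pawn and destroys itself when that pawn overlaps it.
; On overlap it stores its starting location, scale and light intensity, then plays a collection timeline.
; Separate timeline tracks lerp it toward the pawn's live position, scale it to a finish size and fade its point light to zero.
; The actor is destroyed when the timeline finishes.
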(event `self.ReceiveActorBeginOverlap`
  (params (OtherActor :type "Actor Object Reference"))
  ;[1 1 1] Destroy Actor when Collide with Player Pawn / Smoothly travel to the player
  (`self.Is Player` OtherActor
    (:`Is Player`
      (`self.Store Starting Values`)
      (bind (_direction _collection_progress _scale_progress _light_intensity) (`Timeline|Collection Timeline`)
        (:`Update`
          (`self.Move to Player` _collection_progress)
          (`self.Scale Crystals` _scale_progress)
          (`self.Adjust Light` _light_intensity))
        (:`Finished`
          (`self.K2_DestroyActor`))))))

(fn `Adjust Light`
  (params (Alpha :type "Float (double-precision)"))
  (`LightComponent.SetIntensity` (`self.PointLight`) (`KismetMathLibrary.Lerp` (`self.Start Light Intensity`) 0.0 Alpha)))

(fn `Move to Player`
  (params (Alpha :type "Float (double-precision)"))
  (`self.K2_SetActorLocation` (`KismetMathLibrary.VLerp` (`self.Start Location`) (`self.K2_GetActorLocation` (`GameplayStatics.GetPlayerPawn` 0)) Alpha)))

(fn `Scale Crystals`
  (params (Alpha :type "Float (double-precision)"))
  (`self.SetActorScale3D` (`KismetMathLibrary.VLerp` (`self.Start Scale`) (`self.Finish Scale`) Alpha)))

(fn `Store Starting Values`
  (set `self.Start Location` (`self.K2_GetActorLocation`))
  (set `self.Start Scale` (`self.GetActorScale3D`))
  (set `self.Start Light Intensity` (`LightComponentBase.Intensity` (`self.PointLight`))))

(fn `UserConstructionScript`)