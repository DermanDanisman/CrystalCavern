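; Player pawn that moves by applying torque to its mesh and restarts the level when it takes damage.
; Both movement axes lead into one acceleration-change torque call on the mesh, scaled by an acceleration multiplier.
; The camera fades in on BeginPlay.
; The first damage event fades the camera out and holds it, then reopens the current level by name after a short delay.
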(event `InputAxis|Move Forwards/Backwards`
  (params (AxisValue :type "Float (single-precision)"))
  (bind _acceleration_multiplier (`self.Acceleration Multiplier`))
  ;[1 1 1] Movement Controller
  (`PrimitiveComponent.AddTorqueInRadians` (`self.Mesh`) (`KismetMathLibrary.MakeVector` (* (stale `InputAxis|Move RightSide/LeftSide` AxisValue) _acceleration_multiplier) (* AxisValue _acceleration_multiplier)) "None" true :!label _label))

(event `InputAxis|Move RightSide/LeftSide`
  (params (AxisValue :type "Float (single-precision)"))
  ;[1 1 1] Movement Controller
  (goto _label))

(event `self.ReceiveAnyDamage`
  (params (Damage :type "Float (single-precision)") (DamageType :type "DamageType Object Reference") (InstigatedBy :type "Controller Object Reference") (DamageCauser :type "Actor Object Reference"))
  (`/Engine/EditorBlueprintResources/StandardMacros.DoOnce` false
    (:`Completed`
      (`PlayerCameraManager.StartCameraFade` :`self` (`GameplayStatics.GetPlayerCameraManager` 0) :`ToAlpha` 1.0 :`Duration` 1.0 :`bHoldWhenFinished` true)
      (`KismetSystemLibrary.Delay` 1.0)
      (bind _returnvalue (`GameplayStatics.GetCurrentLevelName` true))
      (`GameplayStatics.OpenLevel` (`KismetStringLibrary.Conv_StringToName` _returnvalue)))))

(event `self.ReceiveBeginPlay`
  ;[1 1 1] Camera Fade In
  (`PlayerCameraManager.StartCameraFade` :`self` (`GameplayStatics.GetPlayerCameraManager` 0) :`FromAlpha` 1.0 :`Duration` 3.5))

(fn `UserConstructionScript`)